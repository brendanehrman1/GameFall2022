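; GravityActor is a gravity source meant to pull player characters toward itself through their GravityDirection.
; When a PlayerCharacter leaves the Radius overlap component, its GravityDirection resets to zero.
; The attraction loop, which points overlapping players' GravityDirection at the actor scaled by GravityStrength, is disconnected and never runs.
; Tick is empty, and alternative falloff and base-gravity calculations sit unused.
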(event `self.ReceiveTick`
  (params (DeltaSeconds :type "Float (single-precision)")))

(event `self.Radius.OnComponentEndOverlap`
  (params (OverlappedComponent :type "PrimitiveComponent Object Reference") (OtherActor :type "Actor Object Reference") (OtherComp :type "PrimitiveComponent Object Reference") (OtherBodyIndex :type Integer))
  (cast `CapsuleComponent` OverlappedComponent)
  (bind _asplayer_character (cast `/Game/ThirdPersonBP/Blueprints/PlayerCharacter` OtherActor))
  (set `/Game/ThirdPersonBP/Blueprints/PlayerCharacter.GravityDirection` (0.0 0.0 0.0) _asplayer_character))

(fn `UserConstructionScript`)